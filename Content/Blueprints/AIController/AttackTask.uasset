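; Behavior tree task that makes an AI-controlled unit perform its attack.
; On execute it casts the pawn to UnitBase, calls Attack, resets the Action blackboard enum to its first value and finishes successfully at once.
; A failed cast leaves the task unfinished, the tick event is empty, and an ApplyDamage branch with an AttackTarget lookup is left unused.
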(event EventReceiveExecuteAI
  (params (OwnerController :type AI%20Controller%20Object%20Reference) (ControlledPawn :type Pawn%20Object%20Reference))
  (bind _asunit_base (Utilities|Casting|CastToUnitBase ControlledPawn))
  (bind _output_get (Variables|Default|SetAs%20Unit%20Base _asunit_base))
  (Default|Attack _output_get)
  (Class|BTFunctionLibrary|SetBlackboardValueasEnum (Variables|Default|GetAction))
  (AI|BehaviorTree|FinishExecute true))

(event EventReceiveTickAI
  (params (OwnerController :type AI%20Controller%20Object%20Reference) (ControlledPawn :type Pawn%20Object%20Reference) (DeltaSeconds :type Float%20%28single-precision%29))
  ;[1 1 1] Used so AI can attack in behavior tree
)