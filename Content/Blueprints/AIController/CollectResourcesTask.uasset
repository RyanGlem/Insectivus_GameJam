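; Behavior Tree task that has an AI-controlled unit collect gold from the mine stored in the AttackTarget blackboard key.
; On execute it caches the pawn as a UnitBase, then each tick checks its distance to that UnitMine.
; Within range it fills the unit's carried gold, refreshes the unit frame and finishes successfully.
; Otherwise it resets the Action blackboard enum and keeps running.
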(event EventReceiveExecuteAI
  (params (OwnerController :type AI%20Controller%20Object%20Reference) (ControlledPawn :type Pawn%20Object%20Reference))
  (bind _asunit_base (Utilities|Casting|CastToUnitBase ControlledPawn))
  (Variables|Default|SetAs%20Unit%20Base _asunit_base))

(event EventReceiveTickAI
  (params (OwnerController :type AI%20Controller%20Object%20Reference) (ControlledPawn :type Pawn%20Object%20Reference) (DeltaSeconds :type Float%20%28single-precision%29))
  (bind _as_unit_base (Variables|Default|GetAs%20Unit%20Base))
  ;[1 1 1] Used to collect resources from a mine or a larvae camp and bring them back continously to the base
  (bind _asunit_mine (Utilities|Casting|CastToUnitMine (Class|BTFunctionLibrary|GetBlackboardValueasObject (Variables|Default|GetAttackTarget))))
  (if (<= (Math|Vector|Distance(Vector) (Transformation|GetActorLocation _asunit_mine) (Transformation|GetActorLocation (Variables|Default|GetAs%20Unit%20Base))) 2.1e+02)
    (Variables|/Game/Assets/Units/UnitBase.UnitBase_C|SetGoldCarrying _as_unit_base 10)
    (Default|UpdateUnitFrame _as_unit_base)
    (AI|BehaviorTree|FinishExecute true)
    (else
      (Class|BTFunctionLibrary|SetBlackboardValueasEnum (Variables|Default|GetAction)))))