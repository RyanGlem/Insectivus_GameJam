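; FindUnitBase is an AI behavior tree task that sends a unit back to the main nest to deposit the resources it carries.
; It finds the UnitMainNest actor, moves the controlled unit there, then adds the carried amount to the InsectusGM game mode under the resource type read from the blackboard.
; It then empties the unit's load, refreshes its frame and finishes; only a successful move completes the task.
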(event EventReceiveExecuteAI
  (params (OwnerController :type AI%20Controller%20Object%20Reference) (ControlledPawn :type Pawn%20Object%20Reference))
  (bind _asunit_base (Utilities|Casting|CastToUnitBase ControlledPawn))
  (Variables|Default|SetAs%20Unit%20Base _asunit_base)
  (bind _returnvalue (Actor|GetActorOfClass "/Game/Assets/Units/UnitMainNest.UnitMainNest_C"))
  (Utilities|IsValid ControlledPawn
    (:Is%20Valid
      (AI|AIMoveTo ControlledPawn "0, 0, 0" _returnvalue 5.0 false
        (:OnSuccess
          (bind _asinsectus_gm (Utilities|Casting|CastToInsectusGM (Game|GetGameMode)))
          (Default|AddResource _asinsectus_gm (Variables|/Game/Assets/Units/UnitBase.UnitBase_C|GetResourceCarrying (Variables|Default|GetAs%20Unit%20Base)) (Utilities|Enum|ByteToEnumEResource (Class|BTFunctionLibrary|GetBlackboardValueasEnum (Variables|Default|GetResource))))
          (Variables|/Game/Assets/Units/UnitBase.UnitBase_C|SetResourceCarrying (Variables|Default|GetAs%20Unit%20Base) 0)
          (Default|UpdateUnitFrame (Variables|Default|GetAs%20Unit%20Base))
          (AI|BehaviorTree|FinishExecute true))))))