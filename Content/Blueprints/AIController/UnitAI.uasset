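; UnitAI is an AI controller that runs the UnitBehavior behavior tree for a UnitBase pawn.
; It caches the controlled unit on BeginPlay.
; On successfully sensed perception stimuli, commented as firing when damage is taken, it sets the sensed actor as the unit's TargetActor.
; It then writes the stimulus location and the unit's current Action to the blackboard for the tree to use.
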(event OnTargetPerceptionUpdated(AIPerception)
  (params (Actor :type Actor%20Object%20Reference) (Stimulus :type AI%20Stimulus%20Structure))
  (bind (_age _expirationage _strength _stimuluslocation _receiverlocation _tag _bsuccessfullysensed) (Utilities|Struct|BreakAIStimulus Stimulus))
  (if _bsuccessfullysensed
    (Variables|/Game/Assets/Units/UnitBase.UnitBase_C|SetTargetActor (Variables|Default|GetAs%20Unit%20Base) Actor)
    (AI|Components|Blackboard|SetValueasVector (Variables|Default|GetBlackboard) (Utilities|Name|MakeLiteralName "TargetLocation") _stimuluslocation)
    (AI|Components|Blackboard|SetValueasEnum (Variables|Default|GetBlackboard) (Utilities|Name|MakeLiteralName "EActionEnum") (Variables|/Game/Assets/Units/UnitBase.UnitBase_C|GetAction (Variables|Default|GetAs%20Unit%20Base)))))

(event EventBeginPlay
  (AI|RunBehaviorTree "/Game/Blueprints/AIController/UnitBehavior.UnitBehavior")
  (bind _asunit_base (Utilities|Casting|CastToUnitBase (Pawn|GetControlledPawn)))
  (Variables|Default|SetAs%20Unit%20Base _asunit_base))

(event EventTick
  (params (DeltaSeconds :type Float%20%28single-precision%29)))

(fn ConstructionScript)