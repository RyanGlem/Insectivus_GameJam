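; InsectusController is the player controller for an RTS, handling camera zoom and unit selection input.
; On BeginPlay it locks the mouse to the screen in game-and-UI mode and caches the RTSCamera view target.
; The mouse wheel drives a clamped zoom factor that sets the camera's spring arm length.
; Left mouse press and release message the HUD to start and stop selection, while add and remove functions maintain a duplicate-free UnitSelection array.
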(event EventBeginPlay
  ;[1 1 1] Mouse Lock Mode always clamps mouse to screen so it doesn't leave the screen
  (Input|SetInputModeGameandUI self 0 "LockAlways" false)
  (bind _asrtscamera (Utilities|Casting|CastToRTSCamera (Pawn|GetViewTarget)))
  (Variables|Default|SetRTSCamera _asrtscamera))

(event Input|MouseEvents|MouseWheelAxis
  (params (AxisValue :type Float%20%28single-precision%29))
  (bind _output_get (Variables|Default|SetZoomFactor (Math|Float|Clamp(Float) (+ (* AxisValue -1.0) (Variables|Default|GetZoomFactor)) 0.0 1e+02)))
  (Variables|/Script/Engine.SpringArmComponent|SetTargetArmLength (Variables|/Game/Blueprints/RTSCamera.RTSCamera_C|GetSpringArm (Variables|Default|GetRTSCamera)) (+ (* _output_get 2e+02) 1e+03)))

(event Input|MouseEvents|LeftMouseButton
  (params (Key :type Key%20Structure :default "None"))
  (bind _returnvalue (HUD|GetHUD))
  (:Pressed
    (Class|SelectionInterface|StartSelection(Message) _returnvalue))
  (:Released
    (Class|SelectionInterface|StopSelection(Message) _returnvalue)))

(fn ConstructionScript)

(fn AddUnittoSelection
  (params (UnitBase :type Unit%20Base%20Object%20Reference))
  (Utilities|Array|AddUnique (Variables|Default|GetUnitSelection) UnitBase))

(fn RemoveUnitfromSelection
  (params (UnitBase :type Unit%20Base%20Object%20Reference))
  (Utilities|Array|RemoveItem (Variables|Default|GetUnitSelection) UnitBase))