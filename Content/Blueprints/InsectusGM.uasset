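; InsectusGM, apparently the game mode, tracks the gold and larvae inventories.
; AddResource takes an amount and a resource type, adds to the matching inventory, then broadcasts the new total through the GoldCollected or LarvaeCollected event dispatcher so listening elements can react.
; BeginPlay, Tick and the construction script are empty, and a gold debug print is left unconnected.
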(event EventBeginPlay)

(event EventTick
  (params (DeltaSeconds :type Float%20%28single-precision%29)))

(fn ConstructionScript)

(fn AddResource
  (params (Num :type Integer) (Resource :type EResource%20Enum :default "NewEnumerator0"))
  (switch Utilities|FlowControl|Switch|SwitchonEResource Resource
    (:NewEnumerator0
      (bind _output_get (Variables|Default|SetGoldInventory (+ Num (Variables|Default|GetGoldInventory))))
      (Default|CallGoldCollected _output_get) ; Any time this is called, the element will react to the event dispatcher
    )
    (:NewEnumerator1
      (bind _output_get_2 (Variables|Default|SetLarvaeInventory (+ (Variables|Default|GetLarvaeInventory) Num)))
      (Default|CallLarvaeCollected _output_get_2))))