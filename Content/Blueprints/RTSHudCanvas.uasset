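; RTS HUD class that draws the drag-selection marquee and selects units inside it.
; Interface events start and stop the drag, storing the viewport-scaled mouse position as the first corner.
; While dragging, DrawHUD updates the second corner and, past a minimum diagonal length, draws a translucent rectangle and gathers UnitBase actors within it.
; On release after a marquee, it replaces the InsectusController's unit selection with those actors.
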(event EventBeginPlay
  (bind _asinsectus_controller (Utilities|Casting|CastToInsectusController (Game|GetPlayerController 0)))
  (Variables|Default|SetAs%20Insectus%20Controller _asinsectus_controller))

(event EventStartSelection
  ;[1 1 1] Adding the interface allows us to interact with our HUD from any class freely without casting or calling
  (bind _returnvalue (Class|WidgetLayoutLibrary|GetMousePositiononViewport))
  (Variables|Default|SetPointA (Math|Vector2D|MakeVector2D (.x (* _returnvalue (Class|WidgetLayoutLibrary|GetViewportScale))) (.y (* _returnvalue (Class|WidgetLayoutLibrary|GetViewportScale)))))
  (Variables|Default|SetIsDrawing true) ; Switch to tell us if box is drawing
)

(event EventStopSelection
  (Variables|Default|SetIsDrawing false)
  (if (Variables|Default|GetIsMarquee)
    (Default|ClearUnitSelection (Variables|Default|GetAs%20Insectus%20Controller))
    (for _array_element (Variables|Default|GetSelection%20Of%20Actors)
      (bind _asunit_base (Utilities|Casting|CastToUnitBase _array_element))
      (Default|AddUnittoSelection (Variables|Default|GetAs%20Insectus%20Controller) _asunit_base))
    (Variables|Default|SetIsMarquee false)))

(event EventDrawHUD
  (params (SizeX :type Integer) (SizeY :type Integer))
  (bind _pointa (Variables|Default|GetPointA))
  ;[1 1 1] Adding the interface allows us to interact with our HUD from any class freely without casting or calling
  (if (Variables|Default|GetIsDrawing)
    (bind _returnvalue (Class|WidgetLayoutLibrary|GetMousePositiononViewport))
    (Variables|Default|SetPointB (Math|Vector2D|MakeVector2D (.x (* _returnvalue (Class|WidgetLayoutLibrary|GetViewportScale))) (.y (* _returnvalue (Class|WidgetLayoutLibrary|GetViewportScale))))) ; Gets location of the mouse, sets it to the new mouse position
    (if (> (Math|Vector2D|Vector2DLength (- (Variables|Default|GetPointA) (Variables|Default|GetPointB))) 2e+02)
      (HUD|DrawRect "(R=0.010839,G=0.017589,B=0.316667,A=0.500000)" (.x _pointa) (.y _pointa) (- (.x (Variables|Default|GetPointB)) (.x _pointa)) (- (.y (Variables|Default|GetPointB)) (.y _pointa))) ; Works out the difference between screen width and height
      (Variables|Default|SetIsMarquee true)
      (Variables|Default|SetSelection%20Of%20Actors (Class|HUD|GetActorsinSelectionRectangle "/Game/Assets/Units/UnitBase.UnitBase_C" (Variables|Default|GetPointA) (Variables|Default|GetPointB) true false)))))

(fn ConstructionScript)